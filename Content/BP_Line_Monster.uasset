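; BP_Line_Monster is an enemy that runs along its spline from end to start and can be killed by a bullet.
; It stays hidden until StartMove, then a timeline moves and rotates the mesh along the spline, switching to a looping "pikan" animation on arrival.
; A BP_Bullet hit on the capsule stops movement, plays death, then hides it and disables collision.
; With IsRebirth set, it restarts the run after a delay.
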(event OnComponentHit(Capsule)
  (params (HitComponent :type Primitive%20Component%20Object%20Reference) (OtherActor :type Actor%20Object%20Reference) (OtherComp :type Primitive%20Component%20Object%20Reference) (NormalImpulse :type Vector :default "0, 0, 0") (Hit :type Hit%20Result%20Structure%20%28by%20ref%29))
  (Development|PrintString (Utilities|String|Append "EnemyHit" (Utilities|GetDisplayName OtherActor)))
  (Utilities|Casting|CastToBP_Bullet OtherActor)
  (if (not (Variables|Default|GetIsDie))
    (Variables|Default|SetIsDie true)
    (Utilities|FlowControl|Sequence
      (:then_0
        (Components|Animation|PlayAnimation (Variables|Default|GetSkeletalMesh) "/Game/YHTZ/Animation/dfxb/SM_dfxb_die.SM_dfxb_die" false)
        (Audio|Components|Audio|Stop (Variables|Default|Get时间轴))
        (Utilities|FlowControl|Delay 1.5)
        (Rendering|SetVisibility (Variables|Default|GetSkeletalMesh) false false)
        (Collision|SetCollisionEnabled (Variables|Default|GetCapsule) "NoCollision"))
      (:then_1
        (if (Variables|Default|GetIsRebirth)
          (Utilities|FlowControl|Delay 2.0)
          (Variables|Default|SetIsDie false)
          (Collision|SetCollisionEnabled (Variables|Default|GetCapsule) "QueryOnly")
          (CallFunction|StartMove))))))

(event Custom|StartMove
  (bind _spline (Variables|Default|GetSpline))
  (bind _skeletalmesh (Variables|Default|GetSkeletalMesh))
  (Rendering|SetVisibility (Variables|Default|GetSkeletalMesh) true false)
  (Components|Timeline|SetPlayRate (Variables|Default|Get时间轴) 0.5)
  (Rendering|SetVisibility (Variables|Default|GetSkeletalMesh) true false)
  (Components|Animation|PlayAnimation _skeletalmesh "/Game/YHTZ/Animation/dfxb/SM_dfxb_run.SM_dfxb_run" true)
  (bind _f (Timeline|时间轴 PlayFromStart)
    (:Update
      (Transformation|SetRelativeTransform (Variables|Default|GetSkeletalMesh) (Math|Transform|MakeTransform (.location (Spline|GetTransformatDistanceAlongSpline _spline (Math|Float|Lerp (Spline|GetSplineLength _spline) 0.0 _f) "Local" false)) (Math|Rotator|MakeRotator (.roll (.rotation (Spline|GetTransformatDistanceAlongSpline _spline (Math|Float|Lerp (Spline|GetSplineLength _spline) 0.0 _f) "Local" false))) (.pitch (.rotation (Spline|GetTransformatDistanceAlongSpline _spline (Math|Float|Lerp (Spline|GetSplineLength _spline) 0.0 _f) "Local" false))) (+ (.yaw (.rotation (Spline|GetTransformatDistanceAlongSpline _spline (Math|Float|Lerp (Spline|GetSplineLength _spline) 0.0 _f) "Local" false))) -9e+01)) "1.000000,1.000000,1.000000") false false))
    (:Finished
      (Components|Animation|PlayAnimation _skeletalmesh "/Game/YHTZ/Animation/dfxb/SM_dfxb_pikan.SM_dfxb_pikan" true))))

(event EventBeginPlay
  (Rendering|SetVisibility (Variables|Default|GetSkeletalMesh) false false))

(fn ConstructionScript)