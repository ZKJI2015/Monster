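; BP_DF_XB_A is an actor, apparently an enemy soldier, that dies from a single BP_Bullet hit on its capsule.
; The first hit sets IsDie, swaps the live mesh SMDrxb for the death mesh SMDrxbDie and disables capsule collision.
; After a short delay, IsDieShow decides whether the death mesh stays visible.
; A random roll combined with IsDieShow is left unconnected.
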(event OnComponentHit(Capsule)
  (params (HitComponent :type Primitive%20Component%20Object%20Reference) (OtherActor :type Actor%20Object%20Reference) (OtherComp :type Primitive%20Component%20Object%20Reference) (NormalImpulse :type Vector :default "0, 0, 0") (Hit :type Hit%20Result%20Structure%20%28by%20ref%29))
  (Utilities|Casting|CastToBP_Bullet OtherActor)
  (if (not (Variables|Default|GetIsDie))
    (Variables|Default|SetIsDie true)
    (Rendering|SetVisibility (Variables|Default|GetSM_drxb) false false)
    (Rendering|SetVisibility (Variables|Default|GetSM_drxbDie) true false)
    (Collision|SetCollisionEnabled (Variables|Default|GetCapsule) "NoCollision")
    (Utilities|FlowControl|Delay 0.2)
    (Rendering|SetVisibility (Variables|Default|GetSM_drxbDie) (Variables|Default|GetIsDieShow) false)))

(event EventBeginPlay)

(fn ConstructionScript)